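; AR camera player pawn that streams the device camera's transform over the network.
; BeginPlay starts the AR session, shows the main-frame widget with a mouse cursor, and sets up an ObjectDeliverer UDP sender to a hard-coded address with size-prefixed JSON packets.
; Each Tick copies the camera's world location and rotation into a reused BP_ARCameraData object, sends it, and prints the send result.
; Connect, disconnect and receive handlers are empty.
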(event `self.ReceiveBeginPlay`
  (bind _returnvalue (`GameplayStatics.GetPlayerController` 0))
  (`|ExecutionSequence`
    (:`then_0`
      (`ARBlueprintLibrary.StartARSession` "/Game/ARCameraPlayer/ARSessionConfig.ARSessionConfig"))
    (:`then_1`
      (bind _returnvalue_2 (`|CreateWidget` "/Game/ARCameraPlayer/UI/WBP_PlayerMainFrame.WBP_PlayerMainFrame_C" _returnvalue))
      (`UserWidget.AddToViewport` _returnvalue_2 0)
      (set `PlayerController.bShowMouseCursor` true _returnvalue))
    (:`then_2`
      (`|ExecutionSequence`
        (:`then_0`
          (set `self.MessagingManager` (`ObjectDelivererManager.CreateObjectDelivererManager` true))
          (add `ObjectDelivererManager.Connected` (`self.MessagingManager`) (delegate `Connected_Event`))
          (add `ObjectDelivererManager.Disconnected` (`self.MessagingManager`) (delegate `Disconnected_Event`)))
        (:`then_1`
          (bind _output_get (set `self.MessageBox` (`DeliveryBoxFactory.CreateObjectDeliveryBoxUsingJson` "/Game/ARCameraPlayer/BP_ARCameraData.BP_ARCameraData_C")))
          (add `ObjectDeliveryBoxUsingJson.Received` _output_get (delegate `Received_Event`)))
        (:`then_2`
          (`ObjectDelivererManager.Start` (`self.MessagingManager`) (`ProtocolFactory.CreateProtocolUdpSocketSender` "192.168.31.200") (`PacketRuleFactory.CreatePacketRuleSizeBody` 4 "Little") (`self.MessageBox`)))
        (:`then_3`
          (bind _returnvalue_3 (`|GenericCreateObject` "/Game/ARCameraPlayer/BP_ARCameraData.BP_ARCameraData_C"))
          (set `self.MessageData` _returnvalue_3))))))

(event `Connected_Event`
  (params (ClientSocket :type "ObjectDelivererProtocol Object Reference")))

(event `Disconnected_Event`
  (params (ClientSocket :type "ObjectDelivererProtocol Object Reference")))

(event `Received_Event`
  (params (ReceivedObject :type "Object Object Reference") (ReceivedJsonString :type String) (FromObject :type "ObjectDelivererProtocol Object Reference")))

(event `self.ReceiveTick`
  (params (DeltaSeconds :type "Float (single-precision)"))
  (bind _messagedata (`self.MessageData`))
  (bind _camera (`self.Camera`))
  (set `/Game/ARCameraPlayer/BP_ARCameraData.CameraLocation` (`SceneComponent.K2_GetComponentLocation` _camera) _messagedata)
  (set `/Game/ARCameraPlayer/BP_ARCameraData.CameraRotation` (`SceneComponent.K2_GetComponentRotation` _camera) _messagedata)
  (bind _makedjson (`ObjectDeliveryBoxUsingJson.Send` (`self.MessageBox`) (`self.MessageData`)))
  (`KismetSystemLibrary.PrintString` _makedjson))

(fn `UserConstructionScript`)